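; BP_Bricks is a brick block that BP_Wario can break when he is not small.
; A dive, received through the OnDiveable event, or a hit on the South component destroys it after that size check.
; Hits on the Side component send ChangeDirectionMessage to the other actor, so it can change direction.
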(event OnComponentHit(South)
  (params (HitComponent :type Primitive%20Component%20Object%20Reference) (OtherActor :type Actor%20Object%20Reference) (OtherComp :type Primitive%20Component%20Object%20Reference) (NormalImpulse :type Vector :default "0, 0, 0") (Hit :type Hit%20Result%20Structure%20%28by%20ref%29))
  (bind _asbp_wario (Utilities|Casting|CastToBP_Wario OtherActor))
  (if (not (Default|IsSmall _asbp_wario))
    (Actor|DestroyActor)))

(event OnComponentHit(Side)
  (params (HitComponent :type Primitive%20Component%20Object%20Reference) (OtherActor :type Actor%20Object%20Reference) (OtherComp :type Primitive%20Component%20Object%20Reference) (NormalImpulse :type Vector :default "0, 0, 0") (Hit :type Hit%20Result%20Structure%20%28by%20ref%29))
  (Class|BPIChangeDirection|ChangeDirection(Message) OtherActor))

(event EventOnDiveable
  (params (Player :type BP%20Wario%20Object%20Reference))
  (if (not (Default|IsSmall Player))
    (Actor|DestroyActor)))

(fn ConstructionScript)