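; BP_Poison is a moving poison hazard that sets back the evolution of BP_Wario on contact.
; Each tick it offsets its Sphere along world X by the Direction value, independent of frame time.
; A ChangeDirection event negates Direction to reverse travel, with no caller in this Blueprint.
; When the Sphere begins overlapping BP_Wario, it calls DecrementEvolution on that actor and destroys itself.
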(event OnComponentBeginOverlap(Sphere)
  (params (OverlappedComponent :type Primitive%20Component%20Object%20Reference) (OtherActor :type Actor%20Object%20Reference) (OtherComp :type Primitive%20Component%20Object%20Reference) (OtherBodyIndex :type Integer) (bFromSweep :type Boolean) (SweepResult :type Hit%20Result%20Structure%20%28by%20ref%29))
  (bind _asbp_wario (Utilities|Casting|CastToBP_Wario OtherActor))
  (Default|DecrementEvolution _asbp_wario)
  (Actor|DestroyActor))

(event EventBeginPlay)

(event EventTick
  (params (DeltaSeconds :type Float%20%28single-precision%29))
  (Transformation|AddWorldOffset (Variables|Default|GetSphere) (Math|Vector|MakeVector (Math|Conversions|ToFloat(Integer) (Variables|Default|GetDirection)) 0.0 0.0) false false))

(event EventChangeDirection
  (Variables|Default|SetDirection (* (Variables|Default|GetDirection) -1)))

(fn ConstructionScript)