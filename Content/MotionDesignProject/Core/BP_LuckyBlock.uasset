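; BP_LuckyBlock is a one-shot mystery block that gives either a red mushroom or a coin, depending on its PowerUp flag.
; A South component hit by BP_Wario stores the player, swaps the cube to an activated material, then spawns the mushroom above or calls AddCoin.
; A separate OnHit event does likewise but spawns below and relies on the stored player, as its assignment is unconnected.
; NotActivated, despite its name, becomes true once used.
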(event OnComponentHit(South)
  (params (HitComponent :type Primitive%20Component%20Object%20Reference) (OtherActor :type Actor%20Object%20Reference) (OtherComp :type Primitive%20Component%20Object%20Reference) (NormalImpulse :type Vector :default "0, 0, 0") (Hit :type Hit%20Result%20Structure%20%28by%20ref%29))
  (bind _returnvalue (Transformation|GetActorLocation))
  (if (== false (Variables|Default|GetNotActivated))
    (bind _asbp_wario (Utilities|Casting|CastToBP_Wario OtherActor))
    (Variables|Default|SetActor _asbp_wario)
    (CallFunction|Activated)
    (if (Variables|Default|GetPowerUp)
      (if true
        (Game|SpawnActorfromClass "/Game/MotionDesignProject/Core/BP_Red_Mushroom.BP_Red_Mushroom_C" (Math|Transform|MakeTransform (Math|Vector|MakeVector (.x _returnvalue) (.y _returnvalue) (+ (.z _returnvalue) 9e+01)) "0, 0, 0" "1.000000,1.000000,1.000000") "Undefined" "MultiplyWithRoot" 0 0))
      (else
        (Default|AddCoin (Variables|Default|GetActor))))))

(event Custom|Activated
  (Variables|Default|SetNotActivated true)
  (Rendering|Material|SetMaterial (Variables|Default|GetCube) 0 "/Game/MotionDesignProject/Art/Material/M_Mystery_Activated.M_Mystery_Activated"))

(event EventOnHit
  (params (NewParam :type BP%20Wario%20Object%20Reference))
  (bind _returnvalue (Transformation|GetActorLocation))
  (if (== false (Variables|Default|GetNotActivated))
    (CallFunction|Activated)
    (if (Variables|Default|GetPowerUp)
      (Game|SpawnActorfromClass "/Game/MotionDesignProject/Core/BP_Red_Mushroom.BP_Red_Mushroom_C" (Math|Transform|MakeTransform (Math|Vector|MakeVector (.x _returnvalue) (.y _returnvalue) (+ (.z _returnvalue) -9e+01)) "0, 0, 0" "1.000000,1.000000,1.000000") "Undefined" "MultiplyWithRoot" 0 0)
      (else
        (Default|AddCoin (Variables|Default|GetActor))))))

(fn ConstructionScript)