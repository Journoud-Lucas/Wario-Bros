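; BP_GoalPole is the level's goal flag that ends the game when the player touches it.
; On overlap with the player pawn it tells BP_GameMode to end the game, halves global time dilation and plays the stage-clear sound.
; It also switches Wario's sprite to a flag-catching flipbook matched to his current evolution.
; Hits on its Base component send a change-direction message to the hitting actor, such as an enemy.
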(event OnComponentHit(Base)
  (params (HitComponent :type Primitive%20Component%20Object%20Reference) (OtherActor :type Actor%20Object%20Reference) (OtherComp :type Primitive%20Component%20Object%20Reference) (NormalImpulse :type Vector :default "0, 0, 0") (Hit :type Hit%20Result%20Structure%20%28by%20ref%29))
  ;[0.0152 0.0225 0.1094] Change direction of ennemy who touch the brick
  (Class|BPIChangeDirection|ChangeDirection(Message) OtherActor))

(event Collision|EventActorBeginOverlap
  (params (OtherActor :type Actor%20Object%20Reference))
  (bind _returnvalue (Game|Player|GetPlayerPawn 0))
  ;[0.0152 0.0225 0.1094] End the game when touching the flag
  (if (== OtherActor _returnvalue)
    (bind _asbp_game_mode (Utilities|Casting|CastToBP_GameMode (Game|GetGameMode)))
    (Default|EndtheGame _asbp_game_mode)
    (bind _asbp_wario (Utilities|Casting|CastToBP_Wario _returnvalue))
    (Utilities|Time|SetGlobalTimeDilation 0.5)
    (bind _evolution (Default|GetEvolution _asbp_wario))
    (switch int _evolution
      (:0
        (Sprite|SetFlipbook (Variables|/Script/Paper2D.PaperCharacter|GetSprite _asbp_wario) "/Game/MotionDesignProject/Art/Characters/Wario/WarioSmall/PFB_WarioSmall_CatchFlag.PFB_WarioSmall_CatchFlag"))
      (:1
        (Sprite|SetFlipbook (Variables|/Script/Paper2D.PaperCharacter|GetSprite _asbp_wario) "/Game/MotionDesignProject/Art/Characters/Wario/WarioTall/PFB_WarioTall_CatchFlag.PFB_WarioTall_CatchFlag"))
      (:2
        (Sprite|SetFlipbook (Variables|/Script/Paper2D.PaperCharacter|GetSprite _asbp_wario) "/Game/MotionDesignProject/Art/Characters/Wario/WarioFireBall/PFB_WarioFireBall_CatchFlag.PFB_WarioFireBall_CatchFlag")))
    (Audio|SpawnSound2D "/Game/MotionDesignProject/Sound/A_StageClear.A_StageClear" 1.0 1.0 0.0 0)))

(fn ConstructionScript)