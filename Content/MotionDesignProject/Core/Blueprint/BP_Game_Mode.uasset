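; Game mode that shows the in-game HUD on BeginPlay and handles the end of the game.
; EndTheGame disables player input, shows the mouse cursor and adds the end-game menu widget to the viewport.
; It then casts the player pawn to BP_Wario, zeroes the capsule's physics linear velocity and calls the pawn's own EndTheGame.
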(event Custom|End%20The%20Game
  (bind _returnvalue (Game|Player|GetPlayerPawn 0))
  (bind _returnvalue_2 (Game|GetPlayerController 0))
  (Input|DisableInput _returnvalue _returnvalue_2)
  (Variables|/Script/Engine.PlayerController|SetbShowMouseCursor _returnvalue_2 true)
  (bind _returnvalue_3 (UserInterface|CreateWidget "/Game/MotionDesignProject/UI/Menu/WBP_Menu_EndGame.WBP_Menu_EndGame_C" _returnvalue_2))
  (UserInterface|Viewport|AddtoViewport _returnvalue_3 0)
  (bind _asbp_wario (Utilities|Casting|CastToBP_Wario _returnvalue))
  (Class|PrimitiveComponent|SetAllPhysicsLinearVelocity (Variables|/Script/Engine.Character|GetCapsuleComponent _asbp_wario) "0, 0, 0" false)
  (Default|EndtheGame _asbp_wario))

(event EventBeginPlay
  (bind _returnvalue (UserInterface|CreateWidget "/Game/MotionDesignProject/UI/HUD_Effects/WBP_In_Game_HUD.WBP_In_Game_HUD_C"))
  (UserInterface|Viewport|AddtoViewport _returnvalue 0))

(fn ConstructionScript)