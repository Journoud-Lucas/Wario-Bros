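; BP_Spiny is a walking enemy that damages BP_Wario when its sphere collider hits him.
; It rolls left or right at spawn if Direction is 2, then offsets the sphere along world X each tick, unscaled by delta time, while not dead.
; ChangeDirection reverses movement and rotates the flipbook to match.
; HitbyFireProjectile destroys both the fireball and the Spiny.
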(event OnComponentHit(Sphere)
  (params (HitComponent :type Primitive%20Component%20Object%20Reference) (OtherActor :type Actor%20Object%20Reference) (OtherComp :type Primitive%20Component%20Object%20Reference) (NormalImpulse :type Vector :default "0, 0, 0") (Hit :type Hit%20Result%20Structure%20%28by%20ref%29))
  ;[0.0152 0.0225 0.1094] Damage to wario when hit it (except top)
  (if (not (Variables|Default|GetIsDead))
    (bind _asbp_wario (Utilities|Casting|CastToBP_Wario OtherActor))
    (Default|TakeDamage _asbp_wario)))

(event Custom|Change%20Orientation
  (bind _paperflipbook (Variables|Default|GetPaperFlipbook))
  ;[0.0152 0.0225 0.1094] Change character orientation
  (Math|Float|CompareFloat (Math|Conversions|ToFloat(Integer) (Variables|Default|GetDirection)) 0.0
    (:>
      (Transformation|SetRelativeRotation _paperflipbook "0.000000,180.000000,0.000000" false false))
    (:<
      (Transformation|SetRelativeRotation _paperflipbook "0, 0, 0" false false))))

(event EventBeginPlay
  ;[0.0152 0.0225 0.1094] Random direction at spawn
  (if (== (Variables|Default|GetDirection) 2)
    (if (Math|Random|RandomBool)
      (Variables|Default|SetDirection 1)
      (else
        (Variables|Default|SetDirection -1)))
    (CallFunction|ChangeOrientation)
    (else
      (CallFunction|ChangeOrientation))))

(event EventHitbyFireProjectile
  (params (FireBall :type BP%20Fire%20Projectile%20Object%20Reference))
  ;[0.0152 0.0225 0.1094] Destroy when hit by fireball
  (Actor|DestroyActor FireBall)
  (Actor|DestroyActor))

(event EventTick
  (params (DeltaSeconds :type Float%20%28single-precision%29))
  ;[0.0152 0.0225 0.1094] Movement
  (if (not (Variables|Default|GetIsDead))
    (Transformation|AddWorldOffset (Variables|Default|GetSphere) (Math|Vector|MakeVector (Math|Conversions|ToFloat(Integer) (Variables|Default|GetDirection)) 0.0 0.0) false false)))

(event EventChangeDirection
  ;[0.0152 0.0225 0.1094] Change direction
  (Variables|Default|SetDirection (* (Variables|Default|GetDirection) -1))
  (CallFunction|ChangeOrientation))

(fn ConstructionScript)