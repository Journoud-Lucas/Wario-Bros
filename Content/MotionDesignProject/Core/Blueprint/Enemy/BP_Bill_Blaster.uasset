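; Bill Blaster enemy that periodically fires BP_Bullet_Bill projectiles while its location projects inside the player's viewport.
; Tick gates on visibility and uses a Delay as the fire interval, then spawns a bullet on the matching side and passes it the direction.
; The initial Direction value selects no firing, fixed, random or alternating shots, with the latter two resolved into flags on BeginPlay.
; Hits on the Side component send ChangeDirectionMessage to the other actor.
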(event OnComponentHit(Side)
  (params (HitComponent :type Primitive%20Component%20Object%20Reference) (OtherActor :type Actor%20Object%20Reference) (OtherComp :type Primitive%20Component%20Object%20Reference) (NormalImpulse :type Vector :default "0, 0, 0") (Hit :type Hit%20Result%20Structure%20%28by%20ref%29))
  (Class|BPIChangeDirection|ChangeDirection(Message) OtherActor))

(event EventBeginPlay
  (if (== (Variables|Default|GetDirection) 2)
    ;[0.0152 0.0225 0.1094] Random
    (Variables|Default|Setrandom true)
    (elif (== (Variables|Default|GetDirection) 3)
      (Variables|Default|SetOneOutOfTwo true))))

(event EventTick
  (params (DeltaSeconds :type Float%20%28single-precision%29))
  (if (!= (Variables|Default|GetDirection) 0)
    (if (CallFunction|IsVisibleonScreen)
      (Utilities|FlowControl|Delay 2.0)
      (Utilities|FlowControl|Sequence
        (:then_0
          ;[0.0152 0.0225 0.1094] Random
          (if (== (Variables|Default|Getrandom) true)
            (if (Math|Random|RandomBool)
              (Variables|Default|SetDirection 1)
              (else
                (Variables|Default|SetDirection -1)))))
        (:then_1
          (if (== (Variables|Default|GetOneOutOfTwo) true)
            (if (== (Variables|Default|GetLatestDirection) -1)
              (Variables|Default|SetDirection 1)
              (Variables|Default|SetLatestDirection 1)
              (else
                (Variables|Default|SetDirection -1)
                (Variables|Default|SetLatestDirection -1)))))
        (:then_2
          (if (== (Variables|Default|GetDirection) 1)
            (bind _returnvalue (Game|SpawnActorfromClass "/Game/MotionDesignProject/Core/Blueprint/Enemy/BP_Bullet_Bill.BP_Bullet_Bill_C" (Math|Transform|MakeTransform (Math|Vector|MakeVector 1.5e+02 0.0 1.5e+02) "0, 0, 0" "1.000000,1.000000,1.000000") "Undefined" "MultiplyWithRoot" 0 0))
            (Default|SetDirection _returnvalue (Variables|Default|GetDirection))
            (else
              (bind _returnvalue_2 (Game|SpawnActorfromClass "/Game/MotionDesignProject/Core/Blueprint/Enemy/BP_Bullet_Bill.BP_Bullet_Bill_C" (Math|Transform|MakeTransform (Math|Vector|MakeVector -9e+01 0.0 1.5e+02) "0, 0, 0" "1.000000,1.000000,1.000000") "Undefined" "MultiplyWithRoot" 0 0))
              (Default|SetDirection _returnvalue_2 (Variables|Default|GetDirection)))))))))

(fn ConstructionScript)

(fn IsVisibleonScreen
  (bind _returnvalue (Game|GetPlayerController 0))
  (bind _returnvalue_2 (Transformation|GetActorLocation))
  (bind _returnvalue_3 (Viewport|GetViewportSize))
  (bind _screenlocation (Class|PlayerController|ProjectWorldLocationtoScreen _returnvalue _returnvalue_2 false))
  (return (Math|Boolean|ANDBoolean (> (.x _screenlocation) 0.0) (> (.y _screenlocation) 0.0) (< (.x _screenlocation) (.x _returnvalue_3)) (< (.y _screenlocation) (.y _returnvalue_3)))))