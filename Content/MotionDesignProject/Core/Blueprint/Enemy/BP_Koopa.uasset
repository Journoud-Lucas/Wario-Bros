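; Koopa enemy for a Wario platformer that walks horizontally, frame-rate dependent, and flips its flipbook when reversed.
; Sphere hits damage Wario, while Top hits trigger a timed shell stun that pauses walking and swaps flipbooks before recovery.
; Fireballs, a specific Wario invincibility state, or a dive by non-small Wario destroy it; the dive also awards a coin.
; A sentinel Direction value randomizes the starting direction.
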(event OnComponentHit(Top)
  (params (HitComponent :type Primitive%20Component%20Object%20Reference) (OtherActor :type Actor%20Object%20Reference) (OtherComp :type Primitive%20Component%20Object%20Reference) (NormalImpulse :type Vector :default "0, 0, 0") (Hit :type Hit%20Result%20Structure%20%28by%20ref%29))
  ;[0.0152 0.0225 0.1094] Kill the goomba when Wario hit him by top
  (bind _asbp_wario (Utilities|Casting|CastToBP_Wario OtherActor))
  (switch int (Default|GetInvincible _asbp_wario)
    (:0
      (if (not (Variables|Default|GetIsinshell))
        (Variables|Default|SetIsinshell true)
        (Sprite|SetFlipbook (Variables|Default|GetPaperFlipbook) "/Game/MotionDesignProject/Art/Characters/Enemy/PFB_Koopa_Shell.PFB_Koopa_Shell")
        (Utilities|FlowControl|Delay 2.0)
        (Sprite|SetFlipbook (Variables|Default|GetPaperFlipbook) "/Game/MotionDesignProject/Art/Characters/Enemy/PFB_Koopa_Shell_Up.PFB_Koopa_Shell_Up")
        (Utilities|FlowControl|Delay 2.0)
        (Sprite|SetFlipbook (Variables|Default|GetPaperFlipbook) "/Game/MotionDesignProject/Art/Characters/Enemy/PFB_Koopa.PFB_Koopa")
        (Variables|Default|SetIsinshell false)))
    (:2
      (Actor|DestroyActor))))

(event OnComponentHit(Sphere)
  (params (HitComponent :type Primitive%20Component%20Object%20Reference) (OtherActor :type Actor%20Object%20Reference) (OtherComp :type Primitive%20Component%20Object%20Reference) (NormalImpulse :type Vector :default "0, 0, 0") (Hit :type Hit%20Result%20Structure%20%28by%20ref%29))
  ;[0.0152 0.0225 0.1094] Damage to wario when hit it (except top)
  (bind _asbp_wario (Utilities|Casting|CastToBP_Wario OtherActor))
  (switch int (Default|GetInvincible _asbp_wario)
    (:0
      (Default|TakeDamage _asbp_wario))
    (:2
      (Actor|DestroyActor))))

(event Custom|Change%20Orientation
  (bind _paperflipbook (Variables|Default|GetPaperFlipbook))
  ;[0.0152 0.0225 0.1094] Change character orientation
  (Math|Float|CompareFloat (Math|Conversions|ToFloat(Integer) (Variables|Default|GetDirection)) 0.0
    (:>
      (Transformation|SetRelativeRotation _paperflipbook "0.000000,180.000000,0.000000" false false))
    (:<
      (Transformation|SetRelativeRotation _paperflipbook "0, 0, 0" false false))))

(event EventBeginPlay
  ;[0.0152 0.0225 0.1094] Random direction at spawn
  (if (== (Variables|Default|GetDirection) 2)
    (if (Math|Random|RandomBool)
      (Variables|Default|SetDirection 1)
      (else
        (Variables|Default|SetDirection -1)))
    (CallFunction|ChangeOrientation)
    (else
      (CallFunction|ChangeOrientation))))

(event EventHitbyFireProjectile
  (params (FireBall :type BP%20Fire%20Projectile%20Object%20Reference))
  ;[0.0152 0.0225 0.1094] Destroy when hit by fireball
  (Actor|DestroyActor FireBall)
  (Actor|DestroyActor))

(event EventTick
  (params (DeltaSeconds :type Float%20%28single-precision%29))
  ;[0.0152 0.0225 0.1094] Movement
  (if (not (Variables|Default|GetIsinshell))
    (Transformation|AddWorldOffset (Variables|Default|GetSphere) (Math|Vector|MakeVector (Math|Conversions|ToFloat(Integer) (Variables|Default|GetDirection)) 0.0 0.0) false false)))

(event EventChangeDirection
  ;[0.0152 0.0225 0.1094] Change direction
  (Variables|Default|SetDirection (* (Variables|Default|GetDirection) -1))
  (CallFunction|ChangeOrientation))

(event EventOnDiveable
  (params (Player :type BP%20Wario%20Object%20Reference))
  ;[0.0152 0.0225 0.1094] Kill koopa when dive by big Wario
  (if (not (Default|IsSmall Player))
    (Default|AddCoin Player false)
    (Actor|DestroyActor)))

(fn ConstructionScript)