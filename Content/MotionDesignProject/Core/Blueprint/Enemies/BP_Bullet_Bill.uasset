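; BP_Bullet_Bill is a Bullet Bill enemy that flies in a straight line along X and threatens Wario.
; Direction is set through SetDirection, or randomized to left or right on BeginPlay when it equals 2.
; Tick moves the Box with a swept, fixed per-frame offset.
; Any Box hit destroys the bullet and decrements Wario's evolution, while Wario hitting BoxTop destroys it harmlessly.
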(event OnComponentHit(Box)
  (params (HitComponent :type Primitive%20Component%20Object%20Reference) (OtherActor :type Actor%20Object%20Reference) (OtherComp :type Primitive%20Component%20Object%20Reference) (NormalImpulse :type Vector :default "0, 0, 0") (Hit :type Hit%20Result%20Structure%20%28by%20ref%29))
  ;[0.0152 0.0225 0.1094] Damage to wario when hit it (except top), and destroy actor
  (Actor|DestroyActor)
  (bind _asbp_wario (Utilities|Casting|CastToBP_Wario OtherActor))
  (Default|DecrementEvolution _asbp_wario))

(event OnComponentHit(BoxTop)
  (params (HitComponent :type Primitive%20Component%20Object%20Reference) (OtherActor :type Actor%20Object%20Reference) (OtherComp :type Primitive%20Component%20Object%20Reference) (NormalImpulse :type Vector :default "0, 0, 0") (Hit :type Hit%20Result%20Structure%20%28by%20ref%29))
  ;[0.0152 0.0225 0.1094] Destroy actor when wario hit it by top
  (Utilities|Casting|CastToBP_Wario OtherActor)
  (Actor|DestroyActor))

(event EventBeginPlay
  ;[0.0152 0.0225 0.1094] Random direction at spawn
  (if (== (Variables|Default|GetDirection) 2)
    (if (Math|Random|RandomBool)
      (Variables|Default|SetDirection 1)
      (else
        (Variables|Default|SetDirection -1)))))

(event EventTick
  (params (DeltaSeconds :type Float%20%28single-precision%29))
  ;[0.0152 0.0225 0.1094] Moove every tick
  (Transformation|AddWorldOffset (Variables|Default|GetBox) (Math|Vector|MakeVector (* (Math|Conversions|ToFloat(Integer) (Variables|Default|GetDirection)) 6.0) 0.0 0.0) true false))

(fn ConstructionScript)

(fn SetDirection
  (params (Direction :type Integer))
  ;[0.0152 0.0225 0.1094] Set direction
  (Variables|Default|SetDirection Direction))