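; BP_Poison_Mushroom is a harmful moving pickup that damages BP_Wario on overlap and then destroys itself.
; On BeginPlay, a Direction value of 2 is replaced by a random left or right sign.
; Tick offsets the Sphere along world X by that Direction, without delta-time scaling, so speed depends on frame rate.
; A ChangeDirection event flips the sign, with no caller inside this Blueprint.
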(event OnComponentBeginOverlap(Sphere)
  (params (OverlappedComponent :type Primitive%20Component%20Object%20Reference) (OtherActor :type Actor%20Object%20Reference) (OtherComp :type Primitive%20Component%20Object%20Reference) (OtherBodyIndex :type Integer) (bFromSweep :type Boolean) (SweepResult :type Hit%20Result%20Structure%20%28by%20ref%29))
  ;[0.0152 0.0225 0.1094] Take mushroom
  (bind _asbp_wario (Utilities|Casting|CastToBP_Wario OtherActor))
  (Default|TakeDamage _asbp_wario)
  (Actor|DestroyActor))

(event EventBeginPlay
  ;[0.0152 0.0225 0.1094] Random direction at spawn
  (if (== (Variables|Default|GetDirection) 2)
    (if (Math|Random|RandomBool)
      (Variables|Default|SetDirection 1)
      (else
        (Variables|Default|SetDirection -1)))))

(event EventTick
  (params (DeltaSeconds :type Float%20%28single-precision%29))
  ;[0.0152 0.0225 0.1094] Movement
  (Transformation|AddWorldOffset (Variables|Default|GetSphere) (Math|Vector|MakeVector (Math|Conversions|ToFloat(Integer) (Variables|Default|GetDirection)) 0.0 0.0) false false))

(event EventChangeDirection
  ;[0.0152 0.0225 0.1094] Change direction
  (Variables|Default|SetDirection (* (Variables|Default|GetDirection) -1)))

(fn ConstructionScript)