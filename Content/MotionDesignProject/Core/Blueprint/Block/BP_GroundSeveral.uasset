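; Ground block made of a configurable grid of instanced meshes, which tells actors that hit its Side component to change direction.
; The construction script rebuilds the instances from NumX, NumY and NumZ at fixed spacing, stacking layers downward.
; It then sizes Box to the grid plus a margin, offsetting it along X and Z only.
; On a Side hit, it sends ChangeDirectionMessage to the other actor.
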(event OnComponentHit(Side)
  (params (HitComponent :type Primitive%20Component%20Object%20Reference) (OtherActor :type Actor%20Object%20Reference) (OtherComp :type Primitive%20Component%20Object%20Reference) (NormalImpulse :type Vector :default "0, 0, 0") (Hit :type Hit%20Result%20Structure%20%28by%20ref%29))
  ;[0.0152 0.0225 0.1094] Change direction of the actor who it the block
  (Class|BPIChangeDirection|ChangeDirection(Message) OtherActor))

(fn ConstructionScript
  (bind _numx (Variables|Default|GetNumX))
  (bind _numy (Variables|Default|GetNumY))
  (bind _box (Variables|Default|GetBox))
  (bind _numz (Variables|Default|GetNumZ))
  (bind _returnvalue (Math|Conversions|ToFloat(Integer) _numx))
  (bind _returnvalue_2 (Math|Conversions|ToFloat(Integer) _numy))
  (bind _returnvalue_3 (Math|Conversions|ToFloat(Integer) _numz))
  (bind _returnvalue_4 (Math|Vector|MakeVector _returnvalue _returnvalue_2 _returnvalue_3))
  (Utilities|FlowControl|Sequence
    (:then_0
      (Components|InstancedStaticMesh|ClearInstances (Variables|Default|GetInstancedStaticMesh))
      (for _index (range 0 (- (Variables|Default|GetNumZ) 1))
        (for _index_2 (range 0 (- (Variables|Default|GetNumY) 1))
          (for _index_3 (range 0 (- (Variables|Default|GetNumX) 1))
            (Components|InstancedStaticMesh|AddInstance (Variables|Default|GetInstancedStaticMesh) (Math|Transform|MakeTransform (Math|Vector|MakeVector (* _index_3 100) (* _index_2 100) (* _index -100)) "0, 0, 0" "0.390000,0.390000,0.390000") false)))))
    (:then_1
      (Components|Box|SetBoxExtent _box (+ (* _returnvalue_4 5e+01) 1e+01) true)
      (Transformation|SetRelativeLocation _box (* (* (- _returnvalue_4 1.0) 5e+01) "1.000000,0.000000,-1.000000") false false))))