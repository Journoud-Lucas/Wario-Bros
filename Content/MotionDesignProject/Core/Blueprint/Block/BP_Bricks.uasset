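; Breakable brick block for a Wario platformer that a player who is not small can smash.
; It breaks when hit on its South component by BP_Wario or through the OnDiveable event when dived on, both gated by IsSmall.
; Breaking plays a 2D sound and spawns a Niagara debris effect before destroying the actor.
; Hits on the Side component send ChangeDirectionMessage to the other actor to turn it around.
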(event OnComponentHit(South)
  (params (HitComponent :type Primitive%20Component%20Object%20Reference) (OtherActor :type Actor%20Object%20Reference) (OtherComp :type Primitive%20Component%20Object%20Reference) (NormalImpulse :type Vector :default "0, 0, 0") (Hit :type Hit%20Result%20Structure%20%28by%20ref%29))
  ;[0.0152 0.0225 0.1094] Destroy block when player hit it by south (when he's not small)
  (bind _asbp_wario (Utilities|Casting|CastToBP_Wario OtherActor))
  (if (not (Default|IsSmall _asbp_wario))
    (CallFunction|DestroyActor)))

(event OnComponentHit(Side)
  (params (HitComponent :type Primitive%20Component%20Object%20Reference) (OtherActor :type Actor%20Object%20Reference) (OtherComp :type Primitive%20Component%20Object%20Reference) (NormalImpulse :type Vector :default "0, 0, 0") (Hit :type Hit%20Result%20Structure%20%28by%20ref%29))
  ;[0.0152 0.0225 0.1094] Change direction of the actor who it the block
  (Class|BPIChangeDirection|ChangeDirection(Message) OtherActor))

(event Custom|DestroyActor
  ;[0.0152 0.0225 0.1094] Destroy brick and play sound
  (Audio|PlaySound2D "/Game/MotionDesignProject/Sound/A_Break_Block.A_Break_Block" 1.0 1.0 1.0 0 0)
  (Niagara|SpawnSystematLocation "/Game/MotionDesignProject/Core/FX/NS_Brick_Destroy.NS_Brick_Destroy" (Transformation|GetActorLocation) (Transformation|GetActorRotation) "3.000000,3.000000,3.000000")
  (Actor|DestroyActor))

(event EventOnDiveable
  (params (Player :type BP%20Wario%20Object%20Reference))
  ;[0.0152 0.0225 0.1094] Destroy block when player (when he's not small) dive it
  (if (not (Default|IsSmall Player))
    (CallFunction|DestroyActor)))

(fn ConstructionScript)