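; BP_GameMode is a game mode that manages the in-game HUD and the end-of-game flow.
; On BeginPlay it creates and displays WBP_InGameHUD.
; Its EndTheGame event disables input on the player pawn, shows the mouse cursor, adds the WBP_Menu_EndGame widget, then calls EndTheGame on the BP_Wario pawn.
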(event Custom|End%20The%20Game
  (bind _returnvalue (Game|Player|GetPlayerPawn 0))
  (bind _returnvalue_2 (Game|GetPlayerController 0))
  (Input|DisableInput _returnvalue _returnvalue_2)
  (Variables|/Script/Engine.PlayerController|SetbShowMouseCursor _returnvalue_2 true)
  (bind _returnvalue_3 (UserInterface|CreateWidget "/Game/MotionDesignProject/UI/WBP_Menu_EndGame.WBP_Menu_EndGame_C" _returnvalue_2))
  (UserInterface|Viewport|AddtoViewport _returnvalue_3 0)
  (bind _asbp_wario (Utilities|Casting|CastToBP_Wario _returnvalue))
  (Default|EndtheGame _asbp_wario))

(event EventBeginPlay
  (bind _returnvalue (UserInterface|CreateWidget "/Game/MotionDesignProject/UI/WBP_InGameHUD.WBP_InGameHUD_C"))
  (UserInterface|Viewport|AddtoViewport _returnvalue 0))

(fn ConstructionScript)